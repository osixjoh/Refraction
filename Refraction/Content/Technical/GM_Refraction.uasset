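; Game mode for the Refraction puzzle levels that detects when every receiver is lit and triggers level completion.
; On level load it gathers all B_NewReceiver actors and binds their lit events to a check for any receiver still not receiving.
; When all are lit, it starts the player controller's menu override, shows a completion widget with that level's quote, and unbinds the receiver events.
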(event Custom|All%20Receivers%20Lit
  (bind _aspc_refraction (Utilities|Casting|CastToPC_Refraction (Game|GetPlayerController 0)))
  (Default|CallMenuOverrideStart _aspc_refraction)
  (bind _returnvalue (UserInterface|CreateWidget "/Game/UIWidgets/LevelCompleteWidget.LevelCompleteWidget_C" 0 (Utilities|Array|Get(acopy) (Variables|/Game/Technical/PC_Refraction.PC_Refraction_C|GetLevelQuotes _aspc_refraction) (Variables|/Game/Technical/PC_Refraction.PC_Refraction_C|GetActiveLevel _aspc_refraction))))
  (UserInterface|Viewport|AddtoViewport _returnvalue 0)
  (for _array_element (Variables|Default|GetReceivers)
    (EventDispatchers|UnbindallEventsfromReceiverLit _array_element)))

(event Custom|Level%20Loaded
  (bind _outactors (Actor|GetAllActorsOfClass "/Game/B_NewReceiver.B_NewReceiver_C"))
  (bind _output_get (Variables|Default|SetReceivers _outactors))
  (for _array_element _output_get
    (EventDispatchers|BindEventtoReceiverLit _array_element (delegate Custom|Check%20Receivers))))

(event Custom|Check%20Receivers
  (Variables|Default|SetAnyReceiverUnlit? false)
  (bind _array_element (Utilities|Array|ForEachLoopwithBreak (Variables|Default|GetReceivers) :!label _label)
    (:LoopBody
      (if (not (Variables|/Game/B_NewReceiver.B_NewReceiver_C|GetReceiving _array_element))
        (Variables|Default|SetAnyReceiverUnlit? true)
        (goto _label Break)))
    (:Completed
      (if (not (Variables|Default|GetAnyReceiverUnlit?))
        (CallFunction|AllReceiversLit)))))

(fn ConstructionScript)