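; Player controller for Refraction that runs the main menu, background music and switching between streamed levels.
; BeginPlay shows the menu through the character's MenuCamera, starts persistent music and binds a menu override event that disables click and mouse-over input.
; GoToLevel swaps numbered streamed levels by name and calls MenuToGame, which fades through black, blends to GameCamera, re-enables input and signals the override's end.
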(event Custom|MenuToGame
  (bind _returnvalue (UserInterface|CreateWidget "/Game/UIWidgets/FadeToBlack.FadeToBlack_C"))
  (UserInterface|Viewport|AddtoViewport _returnvalue 0)
  (Utilities|FlowControl|Delay 0.5)
  (Game|Player|SetViewTargetwithBlend (Variables|/Game/TopDownBP/Blueprints/TopDownCharacter.TopDownCharacter_C|GetGameCamera (.AsTop%20Down%20Character (Utilities|Casting|CastToTopDownCharacter (Game|GetPlayerCharacter 0)))) 0.0 "VTBlend_Linear" 0.0 false)
  (Default|FadeOut _returnvalue)
  (Variables|Default|SetbEnableClickEvents true)
  (Variables|Default|SetbEnableMouseOverEvents true)
  (Default|CallMenuOverrideEnd))

(event Custom|BlockGameplay
  (Variables|Default|SetbEnableClickEvents false)
  (Variables|Default|SetbEnableMouseOverEvents false))

(event Custom|Go%20To%20Level
  (params (Level :type Integer))
  ;[1 1 1] Level Loader
  (CallFunction|MenutoGame)
  (Game|UnloadStreamLevel(byName) (Utilities|String|StringToName (Utilities|String|Append "Level" (Utilities|String|ToString(Integer) (Variables|Default|GetActiveLevel)))))
  (Game|LoadStreamLevel(byName) (Utilities|String|StringToName (Utilities|String|Append "Level" (Utilities|String|ToString(Integer) Level))) true)
  (Variables|Default|SetActiveLevel Level))

(event EventBeginPlay
  (bind _returnvalue (UserInterface|CreateWidget "/Game/UIWidgets/MainMenuWidget.MainMenuWidget_C"))
  (UserInterface|Viewport|AddtoViewport _returnvalue 0)
  (Game|Player|SetViewTargetwithBlend (Variables|/Game/TopDownBP/Blueprints/TopDownCharacter.TopDownCharacter_C|GetMenuCamera (.AsTop%20Down%20Character (Utilities|Casting|CastToTopDownCharacter (Game|GetPlayerCharacter 0)))) 0.0 "VTBlend_Linear" 0.0 false)
  (EventDispatchers|BindEventtoMenuOverrideStart (delegate Custom|BlockGameplay))
  (bind _returnvalue_2 (Audio|CreateSound2D "/Game/Sound/SC_BGM.SC_BGM" 1.0 1.0 5.0 0 true false))
  (bind _output_get (Variables|Default|SetBGM _returnvalue_2))
  (Audio|Components|Audio|Play _output_get 5.0))

(fn ConstructionScript)